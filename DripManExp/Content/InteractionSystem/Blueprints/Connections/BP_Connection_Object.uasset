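; BP_Connection_Object is a connection actor in the interaction system whose mesh appears or disappears, and gains or loses collision, as it switches on and off.
; It starts without collision; On enables query and physics collision, and Off disables it.
; BeginPlay, On, Off and SyncInputState all call UpdateState, which flips mesh visibility after the parent update rather than setting it from state.
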(event `self.ReceiveBeginPlay`
  (`parent.ReceiveBeginPlay`)
  (`self.Update State`)
  (`PrimitiveComponent.SetCollisionEnabled` (`self.Mesh`) "NoCollision"))

(event `self.On`
  (`parent.On`)
  (`self.Update State`)
  (`PrimitiveComponent.SetCollisionEnabled` (`self.Mesh`) "QueryAndPhysics"))

(event `self.Off`
  (`parent.Off`)
  (`self.Update State`)
  (`PrimitiveComponent.SetCollisionEnabled` (`self.Mesh`) "NoCollision"))

(event `/Game/InteractionSystem/Core/BPI_Interaction.Sync Input State`
  (params (State :type Boolean))
  (set `self.State` State)
  (`self.Update State`))

(fn `Get Fracture Bool`
  (returns (IsFracture :type Boolean))
  (return false))

(fn `Get Item Type`
  (returns (`Item Type` :type "/Game/InteractionSystem/Core/E_ItemType Enum"))
  (return "NewEnumerator0"))

(fn `Get Mesh`
  (returns (Mesh :type "PrimitiveComponent Object Reference"))
  (return null))

(fn `Update State`
  (`parent.Update State`)
  (`SceneComponent.ToggleVisibility` (`self.Mesh`) false))

(fn `UserConstructionScript`
  (`parent.UserConstructionScript`))